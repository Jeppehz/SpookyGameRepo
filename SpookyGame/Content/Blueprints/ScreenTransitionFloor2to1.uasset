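; A trigger actor that moves the first-person player, apparently from floor 2 to floor 1, behind a screen transition.
; When the player's capsule enters the collision component, it disables input, shows the Fadeout_WBP widget and starts a timer.
; The timer teleports the player to a target location relative to the actor, removes the widget and restores input.
; End overlap clears the timer only if the component still reports overlapping that actor.
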(event `self.ReceiveBeginPlay`
  (bind _asfirst_person_character (cast `/Game/FirstPersonBP/Blueprints/FirstPersonCharacter` (`GameplayStatics.GetPlayerCharacter` 0)))
  (set `self.CharacterRef` _asfirst_person_character))

(event `self.CollisionComponent.OnComponentBeginOverlap`
  (params (OverlappedComponent :type "PrimitiveComponent Object Reference") (OtherActor :type "Actor Object Reference") (OtherComp :type "PrimitiveComponent Object Reference") (OtherBodyIndex :type Integer) (bFromSweep :type Boolean) (SweepResult :type "HitResult Structure (by ref)"))
  (bind _characterref (`self.CharacterRef`))
  (if (== OtherComp (`Character.CapsuleComponent` _characterref))
    (`self.DisableInput` _characterref (`GameplayStatics.GetPlayerController` 0))
    (bind _returnvalue (`KismetSystemLibrary.K2_SetTimerDelegate` (delegate `TeleportToTarget`) (`self.TeleportTime`)))
    (set `self.TeleportTimer` _returnvalue)
    (bind _returnvalue_2 (`|CreateWidget` "/Game/Widgets/Fadeout_WBP.Fadeout_WBP_C"))
    (`UserWidget.AddToViewport` _returnvalue_2 0)))

(event `TeleportToTarget`
  (`self.K2_SetActorLocation` (`self.CharacterRef`) (`KismetMathLibrary.TransformLocation` (`self.GetTransform`) (`self.TargetLocation`)) false false)
  (`Widget.RemoveFromParent` (stale `self.CollisionComponent.OnComponentBeginOverlap` _returnvalue_2))
  (`self.EnableInput` (`self.CharacterRef`) (`GameplayStatics.GetPlayerController` 0)))

(event `self.CollisionComponent.OnComponentEndOverlap`
  (params (OverlappedComponent :type "PrimitiveComponent Object Reference") (OtherActor :type "Actor Object Reference") (OtherComp :type "PrimitiveComponent Object Reference") (OtherBodyIndex :type Integer))
  (if (`PrimitiveComponent.IsOverlappingActor` (`self.CollisionComponent`) OtherActor)
    (`KismetSystemLibrary.K2_ClearAndInvalidateTimerHandle` (`self.TeleportTimer`))))

(fn `UserConstructionScript`)