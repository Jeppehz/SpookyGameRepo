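; Mask pickup actor that grants the player the target item when collected.
; Overlap with MaskHitbox shows or hides a pickup prompt for the FirstPersonCharacter.
; The Disappear event sets HasTargetItem on player 0's character, destroys the actor and adds a PickupNotify_WBP widget to the viewport.
; Nothing in this graph calls Disappear.
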(event `Disappear`
  (bind _asfirst_person_character (cast `/Game/FirstPersonBP/Blueprints/FirstPersonCharacter` (`GameplayStatics.GetPlayerCharacter` 0)))
  (set `/Game/FirstPersonBP/Blueprints/FirstPersonCharacter.HasTargetItem?` true _asfirst_person_character)
  (`self.K2_DestroyActor`)
  (bind _returnvalue (`|CreateWidget` "/Game/Widgets/PickupNotify_WBP.PickupNotify_WBP_C"))
  (bind _output_get (set `self.PickupWidget` _returnvalue))
  (`UserWidget.AddToViewport` _output_get 0))

(event `self.MaskHitbox.OnComponentBeginOverlap`
  (params (OverlappedComponent :type "PrimitiveComponent Object Reference") (OtherActor :type "Actor Object Reference") (OtherComp :type "PrimitiveComponent Object Reference") (OtherBodyIndex :type Integer) (bFromSweep :type Boolean) (SweepResult :type "HitResult Structure (by ref)"))
  (cast `/Game/FirstPersonBP/Blueprints/FirstPersonCharacter` OtherActor)
  (`SceneComponent.SetVisibility` (`self.PickupPrompt`) true false))

(event `self.MaskHitbox.OnComponentEndOverlap`
  (params (OverlappedComponent :type "PrimitiveComponent Object Reference") (OtherActor :type "Actor Object Reference") (OtherComp :type "PrimitiveComponent Object Reference") (OtherBodyIndex :type Integer))
  (cast `/Game/FirstPersonBP/Blueprints/FirstPersonCharacter` OtherActor)
  (`SceneComponent.SetVisibility` (`self.PickupPrompt`) false false))

(fn `UserConstructionScript`)