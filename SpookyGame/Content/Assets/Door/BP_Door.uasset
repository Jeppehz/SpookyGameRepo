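; BP_Door is a swinging door that toggles open and closed when its OpenDoor event is called.
; It caches the first-person player at BeginPlay and uses a dot product against the door's forward vector to pick the swing direction from the player's side.
; A timeline lerps the yaw to open and reverses to close, with a sound for each, marking the door closed only once fully reversed.
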(event `self.ReceiveBeginPlay`
  (bind _asfirst_person_character (cast `/Game/FirstPersonBP/Blueprints/FirstPersonCharacter` (`GameplayStatics.GetPlayerCharacter` 0)))
  (set `self.PlayerRef` _asfirst_person_character))

(event `OpenDoor`
  (bind _scene (`self.Scene`))
  (if (`self.IsDoorClosed?`)
    (set `self.IsDoorClosed?` false)
    (set `self.DotProduct` (`KismetMathLibrary.Dot_VectorVector` (`KismetMathLibrary.Normal` (- (`SceneComponent.K2_GetComponentLocation` _scene) (`self.K2_GetActorLocation` (`self.PlayerRef`)))) (`SceneComponent.GetForwardVector` _scene)))
    (`GameplayStatics.PlaySoundAtLocation` "/Game/Audio/SFX/World/Door/ShortDoorOpen_Cue.ShortDoorOpen_Cue" (`self.K2_GetActorLocation`) (struct) 1.0 1.0 0.0 null null null)
    (bind (_direction _alpha) (`Timeline|OpenDoorTL` :!label _label)
      (:`Update`
        (`SceneComponent.K2_SetRelativeRotation` (`self.Door`) (`KismetMathLibrary.MakeRotator` 0.0 0.0 (`KismetMathLibrary.Lerp` 0.0 (`KismetMathLibrary.SelectFloat` 90.0 -90.0 (>= (`self.DotProduct`) 0.0)) _alpha)) false false))
      (:`Finished`
        (switch `ETimelineDirection` _direction
          (:`Backward`
            (set `self.IsDoorClosed?` true)))))
    (else
      (`GameplayStatics.PlaySoundAtLocation` "/Game/Audio/SFX/World/Door/DoorShut_Cue.DoorShut_Cue" (`self.K2_GetActorLocation`) (struct) 1.0 1.0 0.0 null null null)
      (goto _label :!via `Reverse`))))

(fn `UserConstructionScript`)